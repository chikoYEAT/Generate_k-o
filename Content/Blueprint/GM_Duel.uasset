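; Game mode for a samurai reaction duel between a player and an NPC, run as a phase machine.
; Tick leaves INTRO after a start time, waits a random delay, then enters DRAW, broadcasts the change and shows an exclamation cue.
; A successful attack defeats the opponent, hides the cue and starts a restart timer.
; Separate functions set the FINISH phase or reset both samurai and the phase clock.
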(event `self.ReceiveBeginPlay`
  (bind _returnvalue (`GameplayStatics.GetActorOfClass` "/Game/Blueprint/BP_Exclamation.BP_Exclamation_C"))
  (set `self.Exclamation ref` _returnvalue)
  (bind _returnvalue_2 (`GameplayStatics.GetActorOfClass` "/Game/Blueprint/BP_samorai_player1.BP_samorai_player1_C"))
  (set `self.Samoraiplayer` _returnvalue_2)
  (bind _returnvalue_3 (`GameplayStatics.GetActorOfClass` "/Game/Blueprint/BP_samorai_NPC.BP_samorai_NPC_C"))
  (set `self.SamoraiNPC` _returnvalue_3))

(event `self.ReceiveTick`
  (params (DeltaSeconds :type "Float (single-precision)"))
  (set `self.ElapsedTime` (+ DeltaSeconds (`self.ElapsedTime`)))
  (switch `/Game/Blueprint/Enums/E_Phase` (`self.Phase`)
    (:`NewEnumerator0`
      (if (>= (`self.ElapsedTime`) (`self.RoundStarttime`))
        (set `self.Phase` "NewEnumerator1")
        (`KismetSystemLibrary.Delay` (`KismetMathLibrary.RandomFloatInRange` (`self.Mindrawdelay`) (`self.Maxdrawdelay`)))
        (set `self.Phase` "NewEnumerator2")
        (`self.Drawphasestarted`)
        (`/Engine/EditorBlueprintResources/StandardMacros.IsValid` (`self.Exclamation ref`)
          (:`Is Valid`
            (`/Game/Blueprint/BP_Exclamation.setvisibility` (`self.Exclamation ref`) true))
          (:`Is Not Valid`
            (`KismetSystemLibrary.PrintString` "Exclamation not found")))))))

(fn `AttackedSuccessfully`
  (params (`Is Player` :type Boolean))
  (if `Is Player`
    (`/Game/Blueprint/BP_samorai.Defeated` (`self.SamoraiNPC`))
    (else
      (`/Game/Blueprint/BP_samorai.Defeated` (`self.Samoraiplayer`))))
  (`/Engine/EditorBlueprintResources/StandardMacros.IsValid` (`self.Exclamation ref`)
    (:`Is Valid`
      (`/Game/Blueprint/BP_Exclamation.setvisibility` (`self.Exclamation ref`) false)
      (`KismetSystemLibrary.K2_SetTimerDelegate` (`|CreateDelegate` :!event `Reset`) (`self.RestartDelay`)))))

(fn `Reset`
  (set `self.Phase` "NewEnumerator0")
  (set `self.ElapsedTime` 0.0)
  (`/Game/Blueprint/BP_samorai.Reset` (`self.Samoraiplayer`))
  (`/Game/Blueprint/BP_samorai.Reset` (`self.SamoraiNPC`)))

(fn `SetGameFinished`
  (set `self.Phase` "NewEnumerator3"))

(fn `UserConstructionScript`)