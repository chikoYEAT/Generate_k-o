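; Samurai duelist in a 2D quick-draw duel, usable by player or non-player, with idle, attack and defeated sprites.
; Timelines slide the sprite in on start or reset and lunge it to the attack position.
; Attack allows one press per round: during WAIT it shows a cross as a false start, during DRAW it ends the game.
; Mid-lunge, it swaps to the attack sprite and reports the hit to GM_Duel.
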(event `self.ReceiveBeginPlay`
  (bind _asgm_duel (cast `/Game/Blueprint/GM_Duel` (`GameplayStatics.GetGameMode`)))
  (set `self.Game Mode` _asgm_duel)
  (set `self.Sprite Default Pos` (`SceneComponent.RelativeLocation` (`self.PaperSprite`)))
  (`self.Slidein`)
  (`self.Setcrossvisibility` false))

(event `Defeated`
  (`self.SetSprite` (`self.DefeatedSprite`))
  (`self.Setcrossvisibility` false))

(event `Slidein`
  (`TimelineComponent.SetPlayRate` (`self.SlideinAnum`) 1.0)
  (bind (_direction _alpha) (`Timeline|SlideinAnum` :!via `PlayFromStart`)
    (:`Update`
      (`SceneComponent.K2_SetRelativeLocation` (`self.PaperSprite`) (`KismetMathLibrary.VLerp` (`self.Slide Start Pos`) (`self.Sprite Default Pos`) _alpha) false false))))

(event `Attack`
  (if (not (`self.PressedDraw`))
    (switch `/Game/Blueprint/Enums/E_Phase` (`/Game/Blueprint/GM_Duel.Phase` (`self.Game Mode`))
      (:`NewEnumerator1`
        (`self.Setcrossvisibility` true)
        (set `self.PressedDraw` true))
      (:`NewEnumerator2`
        (set `self.PressedDraw` true)
        (`/Game/Blueprint/GM_Duel.SetGameFinished` (`self.Game Mode`))
        (`TimelineComponent.SetPlayRate` (`self.AttackAnim`) 8.0)
        (bind (_direction _alpha) (`Timeline|AttackAnim` :!via `PlayFromStart`)
          (:`Update`
            (`SceneComponent.K2_SetRelativeLocation` (`self.PaperSprite`) (`KismetMathLibrary.VLerp` (`self.Sprite Default Pos`) (`SceneComponent.RelativeLocation` (`self.AttackPos`)) _alpha) false false))
          (:`Switchsprite`
            (`self.SetSprite` (`self.AttackSprite`))
            (`/Game/Blueprint/GM_Duel.AttackedSuccessfully` (`self.Game Mode`) (`self.IsPlayerControlled`))))))))

(fn `Reset`
  (`self.SetSprite` (`self.IdleSprite`))
  (set `self.PressedDraw` false)
  (`self.Slidein`))

(fn `Setcrossvisibility`
  (params (bNewVisibility :type Boolean))
  (`SceneComponent.SetVisibility` (`self.Cross`) bNewVisibility false))

(fn `SetSprite`
  (params (NewSprite :type "PaperSprite Object Reference"))
  (`PaperSpriteComponent.SetSprite` (`self.PaperSprite`) NewSprite)
  (`PrimitiveComponent.SetMaterial` (`self.PaperSprite`) 0 "/Paper2D/TranslucentUnlitSpriteMaterial.TranslucentUnlitSpriteMaterial")
  (`PrimitiveComponent.SetTranslucentSortPriority` (`self.PaperSprite`) 1))

(fn `UserConstructionScript`)